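; BP_EnemyAttack is a short-lived enemy attack actor that detects whether it reaches the player.
; Tick binds an event to the actor's begin-overlap every frame, counts AttackDuration down by delta time and destroys the actor when it runs out.
; The overlap handler OnOverlapBeguin sets the PlayerReached flag when the other actor is a BP_Player; no damage is applied here.
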(event `self.ReceiveTick`
  (params (DeltaSeconds :type "Float (single-precision)"))
  (add `self.OnActorBeginOverlap` (`|CreateDelegate` :!event `OnOverlapBeguin`))
  (bind _output_get (set `self.attackDuration` (- (`self.attackDuration`) DeltaSeconds)))
  (if (<= _output_get 0.0)
    (`self.K2_DestroyActor`)))

(fn `OnOverlapBeguin`
  (params (OverlappedActor :type "Actor Object Reference") (OtherActor :type "Actor Object Reference"))
  (if (`GameplayStatics.ObjectIsA` OtherActor "/Game/Characters/Player/BP_Player.BP_Player_C")
    (set `self.playerReached` true)))

(fn `UserConstructionScript`
  (`parent.UserConstructionScript`))