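; BP_Enemy is an enemy character with scaffolding for player detection and attacks.
; BeginPlay caches walk speed and the AIC_EnemyController, then binds overlap events on a vision sphere that filter for the player's capsule.
; Detection is unfinished: the line-of-sight trace is disconnected, and neither overlap handler acts on the player.
; TryAttack flags an attack and starts a cooldown that Tick counts down.
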(event `self.ReceiveBeginPlay`
  (bind _visionshpere (`self.VisionShpere`))
  (bind _charactermovement (`self.CharacterMovement`))
  (`|ExecutionSequence`
    (:`then_0`
      (set `self.baseSpeed` (`CharacterMovementComponent.MaxWalkSpeed` _charactermovement))
      (`CharacterMovementComponent.SetMovementMode` _charactermovement "MOVE_Walking" 0)
      (bind _asaic_enemy_controller (cast `/Game/Characters/Enemy/AIC_EnemyController` (`self.GetController`)))
      (set `self.enemyController` _asaic_enemy_controller))
    (:`then_1`
      (`|ExecutionSequence`
        (:`then_0`
          (add `PrimitiveComponent.OnComponentBeginOverlap` _visionshpere (`|CreateDelegate` :!event `OnOverlapBegin`)))
        (:`then_1`
          (add `PrimitiveComponent.OnComponentEndOverlap` _visionshpere (`|CreateDelegate` :!event `OnOverlapEnd`)))))))

(event `self.ReceiveTick`
  (params (DeltaSeconds :type "Float (single-precision)"))
  (`self.UpdateAttackCooldown` DeltaSeconds))

(fn `CheckVisionLine`
  (params (targetActor :type "Actor Object Reference"))
  (returns (obstacleDetected :type Boolean)))

(fn `OnOverlapBegin`
  (params (OverlappedComponent :type "PrimitiveComponent Object Reference") (OtherActor :type "Actor Object Reference") (OtherComp :type "PrimitiveComponent Object Reference") (OtherBodyIndex :type Integer) (bFromSweep :type Boolean) (SweepResult :type "HitResult Structure (by ref)"))
  (bind _enemycontroller (`self.enemyController`)
    (:`then`
      (bind _isplayer (`self.OtherIsPlayer` OtherActor OtherComp))
      (if _isplayer
        (bind _obstacledetected (`self.CheckVisionLine` OtherActor))
        (if (not _obstacledetected)
          (cast `/Game/Characters/Player/BP_Player` OtherActor)
          (set `self.enemyController` _enemycontroller))))
    (:`else`)))

(fn `OnOverlapEnd`
  (params (OverlappedComponent :type "PrimitiveComponent Object Reference") (OtherActor :type "Actor Object Reference") (OtherComp :type "PrimitiveComponent Object Reference") (OtherBodyIndex :type Integer))
  (`self.enemyController`
    (:`then`
      (`self.OtherIsPlayer` OtherActor OtherComp)
      (if true
        _))
    (:`else`)))

(fn `OtherIsPlayer`
  (params (actor :type "Actor Object Reference") (object :type "Object Object Reference"))
  (returns (isPlayer :type Boolean))
  (return (and (`GameplayStatics.ObjectIsA` actor "/Game/Characters/Player/BP_Player.BP_Player_C") (`GameplayStatics.ObjectIsA` object "/Script/Engine.CapsuleComponent"))))

(fn `TryAttack`
  (set `self.attackBegins` true)
  (set `self.attackCooldown` 1.0))

(fn `UpdateAttackCooldown`
  (params (deltaTime :type "Float (double-precision)"))
  (bind _attackcooldown (`self.attackCooldown`))
  (if (> _attackcooldown 0.0)
    (set `self.attackCooldown` (- _attackcooldown deltaTime))))

(fn `UserConstructionScript`)