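; Player character Blueprint that handles jumping with a toggleable double jump and stores the base walk speed.
; IA_Jump drives jump start and stop, while IA_DoubleJump flip-flops the maximum jump count between two and one.
; OnJumped flags a triggered double jump, which is cleared when the jump input completes.
; SetRunning ignores its IsRunning input and always applies base speed, leaving the run multiplier calculation unconnected.
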(event `self.ReceiveBeginPlay`
  (bind _charactermovement (`self.CharacterMovement`))
  (set `self.baseSpeed` (`CharacterMovementComponent.MaxWalkSpeed` _charactermovement))
  (`CharacterMovementComponent.SetMovementMode` _charactermovement "MOVE_Walking" 0))

(event `EnhancedInput|/Game/Character/IA_Jump`
  (params (ActionValue :type Boolean) (ElapsedSeconds :type "Float (double-precision)") (TriggeredSeconds :type "Float (double-precision)") (InputAction :type "InputAction Object Reference" :default "/Game/Character/IA_Jump.IA_Jump"))
  (:`Started`
    (`self.Jump`))
  (:`Completed`
    (`self.StopJumping`)
    (set `self.doubleJumpTriggered` false)))

(event `EnhancedInput|/Game/Character/IA_DoubleJump`
  (params (ActionValue :type Boolean) (ElapsedSeconds :type "Float (double-precision)") (TriggeredSeconds :type "Float (double-precision)") (InputAction :type "InputAction Object Reference" :default "/Game/Character/IA_DoubleJump.IA_DoubleJump"))
  (:`Started`
    (`/Engine/EditorBlueprintResources/StandardMacros.FlipFlop`
      (:`A`
        (set `self.JumpMaxCount` 2))
      (:`B`
        (set `self.JumpMaxCount` 1)))))

(event `self.OnJumped`
  (if (> (`self.JumpCurrentCount`) 1)
    (set `self.doubleJumpTriggered` true)))

(fn `SetRunning`
  (params (isRunning :type Boolean))
  (locals (currentSpeed :type "Float (double-precision)"))
  (`|ExecutionSequence`
    (:`then_0`
      (if true
        (set `local.currentSpeed` (`self.baseSpeed`))))
    (:`then_1`
      (set `CharacterMovementComponent.MaxWalkSpeed` (`local.currentSpeed`) (`self.CharacterMovement`)))))

(fn `UserConstructionScript`)