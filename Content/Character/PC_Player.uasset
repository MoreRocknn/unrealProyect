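; Player controller that turns Enhanced Input into movement, running and camera control for the BP_Player pawn.
; On BeginPlay it sets game-only input, caches the pawn and its camera, and adds the IM_Player mapping context.
; Movement follows the camera's forward and right vectors, directly yawing the mesh toward the travel direction, while IA_Move toggles running while held.
; Camera input rotates the spring arm with scaled speeds and clamped pitch.
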(event `self.ReceiveBeginPlay`
  (`self.INTController`))

(event `EnhancedInput|/Game/Character/IA_Camera`
  (params (ActionValue :type "Vector2D Structure") (ElapsedSeconds :type "Float (double-precision)") (TriggeredSeconds :type "Float (double-precision)") (InputAction :type "InputAction Object Reference" :default "/Game/Character/IA_Camera.IA_Camera"))
  (:`Triggered`
    (`self.MoveCamera` ActionValue)))

(event `EnhancedInput|/Game/Character/IA_Movement`
  (params (ActionValue :type "Vector2D Structure") (ElapsedSeconds :type "Float (double-precision)") (TriggeredSeconds :type "Float (double-precision)") (InputAction :type "InputAction Object Reference" :default "/Game/Character/IA_Movement.IA_Movement"))
  (bind (_x _y) (`KismetMathLibrary.BreakVector2D` ActionValue))
  (:`Triggered`
    (bind _bp_player_ (`self.BP_Player `)
      (:`then`
        (bind _player_cam_ref (`self.Player cam Ref`)
          (:`then`
            (bind _returnvalue (+ (* (`SceneComponent.GetForwardVector` _player_cam_ref) _x) (* (`SceneComponent.GetRightVector` _player_cam_ref) _y)))
            (`Pawn.AddMovementInput` _bp_player_ _returnvalue 1.0 false)
            (bind (_returnvalue_roll _returnvalue_pitch _returnvalue_yaw) (`KismetMathLibrary.BreakRotator` (`KismetMathLibrary.MakeRotFromX` (`KismetMathLibrary.Normal` _returnvalue))))
            (`SceneComponent.K2_SetWorldRotation` (`Character.Mesh` _bp_player_) (`KismetMathLibrary.MakeRotator` 0.0 0.0 (- _returnvalue_yaw 90.0)) false false))
          (:`else`)))
      (:`else`))))

(event `EnhancedInput|/Game/Character/IA_Move`
  (params (ActionValue :type Boolean) (ElapsedSeconds :type "Float (double-precision)") (TriggeredSeconds :type "Float (double-precision)") (InputAction :type "InputAction Object Reference" :default "/Game/Character/IA_Move.IA_Move"))
  (:`Triggered`
    (bind _bp_player_ (`self.BP_Player `)
      (:`then`
        (`/Game/Character/BP_Player.SetRunning` _bp_player_ true))
      (:`else`)))
  (:`Completed`
    (bind _bp_player__2 (`self.BP_Player `)
      (:`then`
        (`/Game/Character/BP_Player.SetRunning` _bp_player__2 false))
      (:`else`))))

(fn `INTController`
  (`WidgetBlueprintLibrary.SetInputMode_GameOnly` self)
  (bind _asbp_player (cast `/Game/Character/BP_Player` (`self.K2_GetPawn`)))
  (bind _output_get (set `self.BP_Player ` _asbp_player))
  (set `self.Player cam Ref` (`/Game/Character/BP_Player.Camera` _output_get))
  (`EnhancedInputSubsystemInterface.AddMappingContext` (subsystem `EnhancedInputLocalPlayerSubsystem`) "/Game/Character/IM_Player.IM_Player" 0 (struct)))

(fn `MoveCamera`
  (params (InVec :type "Vector2D Structure"))
  (bind (_x _y) (`KismetMathLibrary.BreakVector2D` InVec))
  (bind _bp_player_ (`self.BP_Player `)
    (:`then`
      (bind _springarm (`/Game/Character/BP_Player.SpringArm` _bp_player_))
      (`SceneComponent.K2_SetRelativeRotation` _springarm (`KismetMathLibrary.MakeRotator` 0.0 (`KismetMathLibrary.FClamp` (+ (.pitch (`SceneComponent.RelativeRotation` _springarm)) (* _y (`self.camSpeedY`))) (`self.minAngleY`) (`self.maxAngleX`)) (+ (.yaw (`SceneComponent.RelativeRotation` _springarm)) (* _x (`self.camSpeed x`)))) false false))
    (:`else`)))

(fn `UserConstructionScript`)