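; BP_Playerlife tracks a player's life, setting CurrentLife to MaxLife at BeginPlay.
; ReciveDamage sets CurrentLife to Damage minus CurrentLife, the reverse of the usual subtraction order.
; It then broadcasts DamageRecived with the damage amount, followed by OwnerDead if the resulting life is zero or below.
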(event `self.ReceiveBeginPlay`
  (set `self.currentLife` (`self.maxLife`)))

(fn `ReciveDamage`
  (params (Damage :type Integer))
  (bind _output_get (set `self.currentLife` (- Damage (`self.currentLife`))))
  (`|ExecutionSequence`
    (:`then_0`
      (`self.damageRecived` Damage))
    (:`then_1`
      (if (<= _output_get 0)
        (`self.ownerDead`)))))

(fn `UserConstructionScript`)