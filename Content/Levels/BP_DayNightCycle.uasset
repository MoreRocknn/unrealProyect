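; Day-night cycle actor that advances a clock each tick, scaled by a day length in real minutes, and pitches the sun to match.
; It flags night outside hours 6 to 16, comparing it to WasNightTime, which is never updated here, to trigger moon transitions.
; These play or reverse a timeline on the child-actor moon light and toggle its shadows, though each update sets intensity to zero.
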(event `self.ReceiveTick`
  (params (DeltaSeconds :type "Float (single-precision)"))
  (bind _currenthour (`self.CurrentHour`))
  (bind _output_get (set `self.CurrentHour` (+ (`self.CurrentHour`) (* DeltaSeconds (/ 24.0 (* (`self.DayInRealMinutes`) 60.0))))))
  (`|ExecutionSequence`
    (:`then_0`
      (if (>= _output_get 24.0)
        (set `self.CurrentHour` (- (`self.CurrentHour`) 24.0))))
    (:`then_1`
      (`SceneComponent.K2_SetWorldRotation` (`self.Sun`) (`KismetMathLibrary.MakeRotator` 0.0 (- (* (/ (`self.CurrentHour`) 24.0) 360.0) 270.0)) false false))
    (:`then_2`
      (set `self.isNightTime` (or (< _currenthour 6.0) (> _currenthour 16.0)))
      (if (!= (`self.isNightTime`) (`self.WasNightTime`))
        (bind _asdirectional_light (cast `DirectionalLight` (`ChildActorComponent.ChildActor` (`self.Moon`))))
        (if (`self.isNightTime`)
          (bind _lightcomponent (`Light.LightComponent` _asdirectional_light))
          (`LightComponentBase.SetCastShadows` _lightcomponent true)
          (`Timeline|Timeline` :!via `PlayFromStart` :!label _label
            (:`Update`
              (`LightComponent.SetIntensity` _lightcomponent 0.0))
            (:`Finished`
              (if (not (`self.isNightTime`))
                (`LightComponentBase.SetCastShadows` _lightcomponent false))))
          (else
            (goto _label :!via `ReverseFromEnd`)))))
    (:`then_3`
      (set `self.isNightTime` (`self.isNightTime`)))))

(fn `UserConstructionScript`)