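; BP_ActivableDoor is a door that swings open and closed when activated or deactivated, extending a parent activatable-object class.
; It records the closed yaw of SMDoor on BeginPlay, then a timeline scales an opened-rotation offset from that yaw.
; Activation plays the timeline from the start and deactivation reverses it, each guarded by the Activated state before calling the parent implementation.
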(event `self.ReceiveBeginPlay`
  (bind (_relativerotation_roll _relativerotation_pitch _relativerotation_yaw) (`KismetMathLibrary.BreakRotator` (`SceneComponent.RelativeRotation` (`self.SM_Door`))))
  (set `self.closedRotationZ` _relativerotation_yaw))

(event `OpenDoor`
  (bind (_direction _rotation_z) (`Timeline|Timeline` :!via `PlayFromStart` :!label _label)
    (:`Update`
      (`SceneComponent.K2_SetRelativeRotation` (`self.SM_Door`) (`KismetMathLibrary.MakeRotator` 0.0 0.0 (+ (`self.closedRotationZ`) (* _rotation_z (`self.openedRotationZ`)))) false false))))

(event `CloseDoor`
  (goto _label :!via `Reverse`))

(fn `ActivateObject`
  (if (not (`self.activated`))
    (`self.OpenDoor`)
    (`parent.ActivateObject`)))

(fn `DeactivateObject`
  (if (`self.activated`)
    (`self.CloseDoor`)
    (`parent.DeactivateObject`)))

(fn `UserConstructionScript`
  (`parent.UserConstructionScript`))