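; BP_ActivablePlatform is a platform that can be switched on and off, appearing as a solid cube or vanishing completely.
; BeginPlay applies the initial Activated state by toggling the cube's visibility and collision together.
; ActivateObject and DeactivateObject overrides act only on a state change, updating the platform before calling the parent implementation.
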(event `self.ReceiveBeginPlay`
  (if (`self.activated`)
    (`self.EnablePlatform`)
    (else
      (`self.DisablePlatform`))))

(event `EnablePlatform`
  (bind _cube (`self.Cube`))
  (`SceneComponent.SetVisibility` _cube true false)
  (`PrimitiveComponent.SetCollisionEnabled` _cube "QueryAndPhysics"))

(event `DisablePlatform`
  (bind _cube (`self.Cube`))
  (`SceneComponent.SetVisibility` _cube false false)
  (`PrimitiveComponent.SetCollisionEnabled` _cube "NoCollision"))

(fn `ActivateObject`
  (if (not (`self.activated`))
    (`self.EnablePlatform`)
    (`parent.ActivateObject`)))

(fn `DeactivateObject`
  (if (`self.activated`)
    (`self.DisablePlatform`)
    (`parent.DeactivateObject`)))

(fn `UserConstructionScript`
  (`parent.UserConstructionScript`))