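; Activable platform that blinks in and out of existence, flipping its Activated state on a timer of about one second.
; Tick counts down and toggles the state, while BeginPlay applies the initial one.
; Enabling or disabling switches the Cube's visibility and collision together.
; ActivateObject and DeactivateObject overrides also switch the platform when the state differs, then call the parent, but do not pause the timer.
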(event `self.ReceiveTick`
  (params (DeltaSeconds :type "Float (single-precision)"))
  (bind _counter (`self.counter`))
  (bind _activated (`self.activated`))
  (if (<= _counter 0.0)
    (set `self.counter` 1.0)
    (set `self.activated` (not _activated))
    (if _activated
      (`self.EnablePlatform`)
      (else
        (`self.DisablePlatform`)))
    (else
      (set `self.counter` (- _counter DeltaSeconds)))))

(event `self.ReceiveBeginPlay`
  (if (`self.activated`)
    (`self.EnablePlatform`)
    (else
      (`self.DisablePlatform`))))

(event `EnablePlatform`
  (bind _cube (`self.Cube`))
  (`SceneComponent.SetVisibility` _cube true false)
  (`PrimitiveComponent.SetCollisionEnabled` _cube "QueryAndPhysics"))

(event `DisablePlatform`
  (bind _cube (`self.Cube`))
  (`SceneComponent.SetVisibility` _cube false false)
  (`PrimitiveComponent.SetCollisionEnabled` _cube "NoCollision"))

(fn `ActivateObject`
  (if (not (`self.activated`))
    (`self.EnablePlatform`)
    (`parent.ActivateObject`)))

(fn `DeactivateObject`
  (if (`self.activated`)
    (`self.DisablePlatform`)
    (`parent.DeactivateObject`)))

(fn `UserConstructionScript`
  (`parent.UserConstructionScript`))